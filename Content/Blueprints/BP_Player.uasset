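; First-person player character with mouse look, movement, sprint, jump, ledge climb and interaction.
; Jump sphere-traces at eye height; if clear, a downward trace from PlatformChecker seeks a ledge, otherwise the player launches upward.
; Climbing disables input, dips the camera and uses timelines to ease the capsule onto the ledge and restore camera height.
; Capsule overlaps cache INT_Tags actors, which Interact messages through PlayerUseTagMessage.
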(event OnComponentBeginOverlap(CapsuleComponent)
  (params (OverlappedComponent :type Primitive%20Component%20Object%20Reference) (OtherActor :type Actor%20Object%20Reference) (OtherComp :type Primitive%20Component%20Object%20Reference) (OtherBodyIndex :type Integer) (bFromSweep :type Boolean) (SweepResult :type Hit%20Result%20Structure%20%28by%20ref%29))
  (if (Utilities|DoesObjectImplementInterface OtherActor "/Game/Blueprints/INT_Tags.INT_Tags_C")
    (Variables|Default|SetTaggableObject OtherActor)
    (Variables|Default|SetCanTag? true)))

(event OnComponentEndOverlap(CapsuleComponent)
  (params (OverlappedComponent :type Primitive%20Component%20Object%20Reference) (OtherActor :type Actor%20Object%20Reference) (OtherComp :type Primitive%20Component%20Object%20Reference) (OtherBodyIndex :type Integer))
  (if (Utilities|DoesObjectImplementInterface OtherActor "/Game/Blueprints/INT_Tags.INT_Tags_C")
    (Variables|Default|SetTaggableObject 0)
    (Variables|Default|SetCanTag? false)))

(event EventBeginPlay
  ;[1 1 1] Begin play
  (Variables|Default|SetWalkSpeed (Variables|/Script/Engine.CharacterMovementComponent|GetMaxWalkSpeed (Variables|Character|GetCharacterMovement))))

(event Input|ActionEvents|InputActionJump
  (params (Key :type Key%20Structure :default "None"))
  (bind _returnvalue (Transformation|GetVelocity))
  ;[1 1 1] Jump & Ledge Climb
  (:Pressed
    (if (not (Variables|Default|GetMovementDisabled))
      (bind _blockedsight_ (CallFunction|EyeHeightCheck))
      (if _blockedsight_
        _
        (else
          (bind _platformlocation (CallFunction|ClimbUp))))
      (if (Variables|Default|GetMovementDisabled)
        ;[1 0.8424 0.6533] Move the player up to platform
        (Variables|Default|SetPlatform%20Location _platformlocation)
        (bind _climb (Timeline|PlayeClimb PlayFromStart)
          (:Update
            (Transformation|SetWorldLocation (Variables|Collision|GetCapsuleComponent) (Math|Interpolation|Ease "EaseInOut" _climb (Transformation|GetWorldLocation (Variables|Collision|GetCapsuleComponent)) (Variables|Default|GetPlatform%20Location) 2.0) false false)
            ;[1 0.3625 0.4122] Move Camera to Original height
            (bind _reseteyeheight (Timeline|ResetEyeHeight Play)
              (:Update
                (Transformation|SetRelativeLocation (Variables|Default|GetPlayerCamera) (Math|Interpolation|Ease "Linear" _reseteyeheight (Variables|/Script/Engine.SceneComponent|GetRelativeLocation (Variables|Default|GetPlayerCamera)) (Math|Vector|MakeVector 0.0 0.0 75.0)) false false))
              (:Finished
                (Variables|/Script/Engine.MovementComponent|SetVelocity (Variables|Character|GetCharacterMovement) (Math|Vector|MakeVector 0.0 0.0 0.0))
                (Variables|Default|SetMovementDisabled false)))))
        (elif (not (AI|Components|NavMovement|IsFalling (Variables|Character|GetCharacterMovement)))
          (Character|LaunchCharacter (Math|Vector|MakeVector (.x _returnvalue) (.y _returnvalue) (+ (.z _returnvalue) (Variables|Default|GetJumpHeight))) true true)
          (Variables|Default|SetMovementDisabled false))))))

(event Input|ActionEvents|InputActionSprint
  (params (Key :type Key%20Structure :default "None"))
  (bind _charactermovement (Variables|Character|GetCharacterMovement))
  ;[1 1 1] Sprint
  (:Pressed
    (Variables|/Script/Engine.CharacterMovementComponent|SetMaxWalkSpeed _charactermovement (Variables|Default|GetRunSpeed)))
  (:Released
    (Variables|/Script/Engine.CharacterMovementComponent|SetMaxWalkSpeed _charactermovement (Variables|Default|GetWalkSpeed))))

(event Input|ActionEvents|InputActionInteract
  (params (Key :type Key%20Structure :default "None"))
  (:Pressed
    (if (Variables|Default|GetCanTag?)
      (Class|INTTags|PlayerUseTag(Message) (Variables|Default|GetTaggableObject)))))

(event Input|AxisEvents|InputAxisMoveForward
  (params (AxisValue :type Float%20%28single-precision%29))
  ;[1 1 1] Basic Movement
  (if (not (Variables|Default|GetMovementDisabled))
    (Pawn|Input|AddMovementInput (Math|Vector|GetForwardVector (Math|Rotator|MakeRotator 0.0 0.0 (.yaw (Pawn|GetControlRotation :!class /Script/Engine.Pawn)))) AxisValue false)))

(event Input|AxisEvents|InputAxisMoveRIght
  (params (AxisValue :type Float%20%28single-precision%29))
  ;[1 1 1] Basic Movement
  (if (not (Variables|Default|GetMovementDisabled))
    (Pawn|Input|AddMovementInput (Math|Vector|GetRightVector (Math|Rotator|MakeRotator 0.0 0.0 (.yaw (Pawn|GetControlRotation :!class /Script/Engine.Pawn)))) AxisValue false)))

(event Input|AxisEvents|InputAxisLookRight
  (params (AxisValue :type Float%20%28single-precision%29))
  ;[1 1 1] Basic Mouse Look
  (if (not (Variables|Default|GetMovementDisabled))
    (Pawn|Input|AddControllerYawInput AxisValue)))

(event Input|AxisEvents|InputAxisLookUp
  (params (AxisValue :type Float%20%28single-precision%29))
  ;[1 1 1] Basic Mouse Look
  (if (not (Variables|Default|GetMovementDisabled))
    (Pawn|Input|AddControllerPitchInput AxisValue)))

(fn ConstructionScript)

(fn EyeHeightCheck
  (bind _eyes (Variables|Default|GetEyes))
  (bind _returnvalue (Transformation|GetWorldTransform _eyes))
  (bind _returnvalue_2 (Collision|SphereTraceForObjects (.location _returnvalue) (+ (.location _returnvalue) (* (Math|Vector|GetForwardVector (.rotation _returnvalue)) (Variables|Default|GetEyeTraceLength))) 1e+01 (Utilities|Array|MakeArray "ObjectTypeQuery1") false 0 "ForDuration"))
  (if _returnvalue_2
    (Development|PrintString "Sight is blocked")
    (Variables|Default|SetSightBlocked? true)
    (else
      (Development|PrintString "Sight is free")
      (Variables|Default|SetSightBlocked? false)))
  (return (Variables|Default|GetSightBlocked?)))

(fn ClimbUp
  (bind _playercamera (Variables|Default|GetPlayerCamera))
  (bind _platformchecker (Variables|Default|GetPlatformChecker))
  (bind _returnvalue (Transformation|GetWorldTransform _platformchecker))
  (bind (_outhit _returnvalue_2) (Collision|SphereTraceForObjects (.location _returnvalue) (+ (.location _returnvalue) (* (* (Math|Vector|GetUpVector (.rotation _returnvalue)) (Math|Vector|VectorDown)) (Variables|Default|GetLocationTraceLength))) 1e+01 (Utilities|Array|MakeArray "ObjectTypeQuery1") false 0 "ForDuration"))
  (if _returnvalue_2
    (Variables|Default|SetMovementDisabled true)
    (Transformation|SetRelativeLocation _playercamera (/ (Variables|/Script/Engine.SceneComponent|GetRelativeLocation _playercamera) 2) false false) ; Moving the player camera down a little
    (return (Math|Vector|MakeVector (.x (.Location (Collision|BreakHitResult _outhit))) (.y (.Location (Collision|BreakHitResult _outhit))) (+ (.z (.Location (Collision|BreakHitResult _outhit))) (Components|Capsule|GetScaledCapsuleHalfHeight (Variables|Collision|GetCapsuleComponent)))))))