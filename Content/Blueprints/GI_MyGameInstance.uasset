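; GI_MyGameInstance is a game instance that tracks how many paintings the player has tagged.
; UpdateTotalTags stores the level's painting total, resets the tagged count and prints the total.
; UpdateCurrentTags increments the count and prints either the running tally or an all-tagged message when it matches the total.
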(event EventUpdateTotalTags
  (params (NewParam :type Integer))
  ;[1 1 1] Level Start
  (Variables|Default|SetTotalPaintings NewParam)
  (Variables|Default|SetTotalTags 0)
  (Development|PrintString (Utilities|String|ToString(Integer) (Variables|Default|GetTotalPaintings))))

(event EventUpdateCurrentTags
  ;[1 1 1] Check if all paintings have been tagged or not
  (bind _result (Math|Integer|IncrementInt (Variables|Default|GetTotalTags))
    (:%20%20
      (if (== _result (Variables|Default|GetTotalPaintings))
        (Development|PrintString "ALL PAINTINGS TAGGED!")
        (else
          (Development|PrintString (Utilities|String|Append "Paintings Tagged = " (Utilities|String|ToString(Integer) (Variables|Default|GetTotalTags)))))))))