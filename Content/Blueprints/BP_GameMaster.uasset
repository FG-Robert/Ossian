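; BP_GameMaster tracks how many of the level's paintings have been tagged.
; On BeginPlay it counts every actor tagged "Painting", passing the running total to the Game Instance through UpdateTotalTagsMessage.
; Each UpdateTotalTags call increments the tag count and compares it to the painting total.
; It prints the current count, or an all-tagged message when the two match, with no other completion logic.
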(event EventBeginPlay
  ;[1 1 1] GET TOTAL AMOUNT OF PAINTINGS IN THE LEVEl
  (bind _outactors (Actor|GetAllActorswithTag "Painting"))
  (for _array_element _outactors
    (bind _result (Math|Integer|IncrementInt (Variables|Default|GetTotalPaintings))
      (:%20%20
        (Class|INTGameMaster|UpdateTotalTags(Message) (Game|GetGameInstance) _result)))))

(event EventUpdateTotalTags
  (params (NewParam :type Integer))
  ;[1 1 1] Update total tags and check if it is the same as amount of paintings
  (bind _result (Math|Integer|IncrementInt (Variables|Default|GetTotalTags))
    (:%20%20
      (bind _output_get (Variables|Default|SetTotalTags _result))
      (if (== _output_get (Variables|Default|GetTotalPaintings))
        (Development|PrintString "ALL PAINTINGS TAGGED!")
        (else
          (Development|PrintString (Utilities|String|ToString(Integer) (Variables|Default|GetTotalTags))))))))

(fn ConstructionScript)