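; BP_Tag is a tag Blueprint that reveals itself in a random colour when its ShowTag event is called.
; ShowTag creates a dynamic instance of Mat_Tag_Master, randomises its Colour parameter within a range that avoids very dark channels, and applies it to the Tag component.
; It then unhides DefaultSceneRoot and all its children in game.
; The construction script is empty.
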(event EventShowTag
  (bind _returnvalue (Rendering|Material|CreateDynamicMaterialInstance "/Game/Materials/Mat_Tag_Master.Mat_Tag_Master" "None" "None" :!class /Script/Engine.KismetMaterialLibrary))
  (Variables|Default|SetDynamicMaterial _returnvalue)
  (Rendering|Material|SetVectorParameterValue (Variables|Default|GetDynamicMaterial) "Colour" (Utilities|Struct|MakeLinearColor (Math|Random|RandomFloatinRange 0.2 1.0) (Math|Random|RandomFloatinRange 0.2 1.0) (Math|Random|RandomFloatinRange 0.2 1.0) 1.0) :!class /Script/Engine.MaterialInstanceDynamic)
  (Rendering|Material|SetMaterial (Variables|Default|GetTag) 0 (Variables|Default|GetDynamicMaterial))
  (Development|SetHiddeninGame (Variables|Default|GetDefaultSceneRoot) false true))

(fn ConstructionScript)